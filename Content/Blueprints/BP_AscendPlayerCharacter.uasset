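; Player character Blueprint that connects to the Ascend ability system and reports landings as gameplay events.
; BeginPlay grants the default ability set with automatic runtime slot assignment turned off.
; Pressing F manually assigns default slots for the granted abilities and prints the result.
; On landing, it sends itself a Landed gameplay event carrying the custom jump cooldown as event magnitude.
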(event EventBeginPlay
  (bind _defaultabilityset (Variables|Ability|GetDefaultAbilitySet)
    (:then
      (bind _abilitysystem (Class|AscendAbilitySystemComponent|TryGetAscendAbilitySystem self)
        (:True
          (Class|AscendAbilitySet|GivetoAbilitySystem _defaultabilityset _abilitysystem self false))))
    (:else)))

(event EventOnLanded
  (params (Hit :type Hit%20Result%20Structure%20%28by%20ref%29))
  (bind _self self)
  (bind _structout (Utilities|Struct|SetmembersinGameplayEventData (Variables|Events|GetOnLandedPayload) _self (Variables|Default|GetCustomJumpCooldown)))
  (Ability|SendGameplayEventtoActor _self "(TagName=\"GameplayEvent.Landed\")" _structout))

(event Input|KeyboardEvents|F
  (params (Key :type Key%20Structure :default "None"))
  (:Pressed
    ;[0.15 0.15 0.15 0.5] If AutoAssign is not checked as true when the Ability Set is issued, automatic assignment must be done manually.
    (bind _abilitysystem (Class|AscendAbilitySystemComponent|TryGetAscendAbilitySystem self)
      (:True
        (bind _returnvalue (Class|AscendAbilitySystemComponent|AutoAssignDefaultSlotsforGrantedAbilities _abilitysystem true))
        (Development|PrintString (Utilities|String|ToString(Integer) _returnvalue))))))

(fn ConstructionScript)