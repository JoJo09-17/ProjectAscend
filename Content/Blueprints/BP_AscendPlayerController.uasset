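; Player controller that builds the root HUD layout, binds it to the pawn's Ascend ability system, and handles movement input.
; IA_Move drives the controlled pawn along control-rotation forward and right vectors.
; Hard-wired numpad keys auto-assign granted abilities or, via MoveSlot, put the tag-found LeapSlam ability into one of three slots.
; Other hard-wired keys apply mana-reset and attack-speed effects to the pawn, apparently for testing.
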(event Input|EnhancedActionEvents|EnhancedInputActionIA_Move
  (params (ActionValue :type Vector%202D%20Structure) (ElapsedSeconds :type Float%20%28double-precision%29) (TriggeredSeconds :type Float%20%28double-precision%29) (InputAction :type Input%20Action%20Object%20Reference :default "/Game/Input/Actions/IA_Move.IA_Move"))
  (bind _returnvalue (Pawn|GetControlledPawn))
  (bind (_x _y) (Math|Vector2D|BreakVector2D ActionValue))
  (bind _returnvalue_2 (Pawn|GetControlRotation :!class /Script/Engine.Controller))
  (Pawn|Input|AddMovementInput _returnvalue (Math|Vector|GetForwardVector (Math|Rotator|MakeRotator 0.0 0.0 (.yaw (Pawn|GetControlRotation :!class /Script/Engine.Controller)))) _x false)
  (Pawn|Input|AddMovementInput _returnvalue (Math|Vector|GetRightVector (Math|Rotator|MakeRotator (.roll _returnvalue_2) 0.0 (.yaw _returnvalue_2))) _y false))

(event EventBeginPlay
  (bind _returnvalue (UserInterface|CreateWidget "/Game/UI/WBP_RootLayout.WBP_RootLayout_C" self))
  (UserInterface|Viewport|AddtoViewport _returnvalue 0)
  (bind _abilitysystem (Class|AscendAbilitySystemComponent|TryGetAscendAbilitySystem (Pawn|GetControlledPawn))
    (:True
      (Default|InitializeAbilitySystem _returnvalue _abilitysystem))))

(event Input|KeyboardEvents|Add
  (params (Key :type Key%20Structure :default "None"))
  (:Pressed
    (bind _abilitysystem (Class|AscendAbilitySystemComponent|TryGetAscendAbilitySystem (Pawn|GetControlledPawn))
      (:True
        (GameplayEffects|ApplyGameplayEffectToSelf :self _abilitysystem :GameplayEffectClass "/Game/Blueprints/AbilitySystem/GameplayEffects/GE_AttackSpeedIncrease.GE_AttackSpeedIncrease_C")))))

(event Input|KeyboardEvents|NumPadZero
  (params (Key :type Key%20Structure :default "None"))
  (:Pressed
    (Class|AscendAbilitySlotComponent|AutoAssignGrantedAbilities (Class|AscendPlayerController|GetAbilitySlotComponent) true)))

(event Input|KeyboardEvents|NumPadTwo
  (params (Key :type Key%20Structure :default "None"))
  (:Pressed
    (CallFunction|MoveSlot "(TagName=\"InputTag.Ability.Slot2\")")))

(event Input|KeyboardEvents|NumPadOne
  (params (Key :type Key%20Structure :default "None"))
  (:Pressed
    (CallFunction|MoveSlot "(TagName=\"InputTag.Ability.Slot1\")")))

(event Input|KeyboardEvents|NumPadThree
  (params (Key :type Key%20Structure :default "None"))
  (:Pressed
    (CallFunction|MoveSlot "(TagName=\"InputTag.Ability.Slot3\")")))

(event Input|KeyboardEvents|R
  (params (Key :type Key%20Structure :default "None"))
  (:Pressed
    (bind _abilitysystem (Class|AscendAbilitySystemComponent|TryGetAscendAbilitySystem (Pawn|GetControlledPawn))
      (:True
        (GameplayEffects|ApplyGameplayEffectToSelf :self _abilitysystem :GameplayEffectClass "/Game/Blueprints/AbilitySystem/GameplayEffects/GE_ResetMana.GE_ResetMana_C")))))

(fn ConstructionScript)

(fn MoveSlot
  (params (SlotTag :type Gameplay%20Tag%20Structure))
  (bind _abilitysystem (Class|AscendAbilitySystemComponent|TryGetAscendAbilitySystem (Pawn|GetControlledPawn))
    (:True
      (Class|AscendAbilitySystemComponent|AssignAbilitytoSlot _abilitysystem (.OutAbilityHandle (Class|AscendAbilityQueryLibrary|FindAbilityHandlebyTag _abilitysystem (GameplayTags|MakeLiteralGameplayTag "(TagName=\"Ability.Type.Action.LeapSlam\")"))) SlotTag (.ReturnValue (Class|AscendAbilityQueryLibrary|FindAbilityHandlebyTag _abilitysystem (GameplayTags|MakeLiteralGameplayTag "(TagName=\"Ability.Type.Action.LeapSlam\")")))))))